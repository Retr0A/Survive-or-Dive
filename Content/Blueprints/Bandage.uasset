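; Bandage pickup that heals the player by one health point when Interact is pressed.
; A sphere overlap enables input and sets a HUD prompt through MainGameMode, with a different message at full health (4); leaving disables input and clears it.
; Interacting destroys both meshes rather than the actor, plays a sound and updates the HUD health, with the mesh validity checks preventing reuse.
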(event OnComponentEndOverlap(Sphere)
  (params (OverlappedComponent :type Primitive%20Component%20Object%20Reference) (OtherActor :type Actor%20Object%20Reference) (OtherComp :type Primitive%20Component%20Object%20Reference) (OtherBodyIndex :type Integer))
  (if (== OtherActor (Game|GetPlayerCharacter 0))
    (Input|DisableInput (Game|GetPlayerController 0))
    (bind _asmain_game_mode (Utilities|Casting|CastToMainGameMode (Game|GetGameMode)))
    (Variables|/Game/UI/HeadsUpDisplay.HeadsUpDisplay_C|SetMessage (Variables|/Game/GameSettings/MainGameMode.MainGameMode_C|GetHeadsUpDisplay _asmain_game_mode) "")
    (Default|UpdateMessage (Variables|/Game/GameSettings/MainGameMode.MainGameMode_C|GetHeadsUpDisplay _asmain_game_mode))))

(event OnComponentBeginOverlap(Sphere)
  (params (OverlappedComponent :type Primitive%20Component%20Object%20Reference) (OtherActor :type Actor%20Object%20Reference) (OtherComp :type Primitive%20Component%20Object%20Reference) (OtherBodyIndex :type Integer) (bFromSweep :type Boolean) (SweepResult :type Hit%20Result%20Structure%20%28by%20ref%29))
  (bind _staticmesh (Variables|Default|GetStaticMesh))
  (if (== OtherActor (Game|GetPlayerCharacter 0))
    (bind _asplayer_character (Utilities|Casting|CastToPlayerCharacter (Game|GetPlayerCharacter 0)))
    (if (== (Variables|/Game/Characters/PlayerCharacter.PlayerCharacter_C|GetHealth _asplayer_character) 4)
      (Input|EnableInput 0)
      (Utilities|IsValid _staticmesh
        (:Is%20Valid
          (Utilities|IsValid _staticmesh
            (:Is%20Valid
              (bind _asmain_game_mode (Utilities|Casting|CastToMainGameMode (Game|GetGameMode)))
              (Variables|/Game/UI/HeadsUpDisplay.HeadsUpDisplay_C|SetMessage (Variables|/Game/GameSettings/MainGameMode.MainGameMode_C|GetHeadsUpDisplay _asmain_game_mode) "You have full health!")
              (Default|UpdateMessage (Variables|/Game/GameSettings/MainGameMode.MainGameMode_C|GetHeadsUpDisplay _asmain_game_mode))))))
      (else
        (Input|EnableInput (Game|GetPlayerController 0))
        (Utilities|IsValid (Variables|Default|GetStaticMesh)
          (:Is%20Valid
            (Utilities|IsValid (Variables|Default|GetStaticMesh1)
              (:Is%20Valid
                (bind _asmain_game_mode_2 (Utilities|Casting|CastToMainGameMode (Game|GetGameMode)))
                (Variables|/Game/UI/HeadsUpDisplay.HeadsUpDisplay_C|SetMessage (Variables|/Game/GameSettings/MainGameMode.MainGameMode_C|GetHeadsUpDisplay _asmain_game_mode_2) "Press [E] to heal with the bandage.")
                (Default|UpdateMessage (Variables|/Game/GameSettings/MainGameMode.MainGameMode_C|GetHeadsUpDisplay _asmain_game_mode_2))))))))))

(event EventBeginPlay)

(event Collision|EventActorBeginOverlap
  (params (OtherActor :type Actor%20Object%20Reference)))

(event EventTick
  (params (DeltaSeconds :type Float%20%28single-precision%29)))

(event Input|ActionEvents|InputActionInteract
  (params (Key :type Key%20Structure :default "None"))
  (bind _returnvalue (Game|GetPlayerCharacter 0))
  (bind _staticmesh (Variables|Default|GetStaticMesh))
  (:Pressed
    (Utilities|IsValid _staticmesh
      (:Is%20Valid
        (Utilities|IsValid (Variables|Default|GetStaticMesh1)
          (:Is%20Valid
            (Components|DestroyComponent _staticmesh)
            (Audio|PlaySoundatLocation "/Game/Sounds/Pickup.Pickup" (Transformation|GetActorLocation _returnvalue) "0, 0, 0" 1.0 1.0 0.0 0 0 0)
            (bind _asplayer_character (Utilities|Casting|CastToPlayerCharacter _returnvalue))
            (Math|Integer|IncrementInt (Variables|/Game/Characters/PlayerCharacter.PlayerCharacter_C|GetHealth _asplayer_character)
              (:%20%20
                (bind _asmain_game_mode (Utilities|Casting|CastToMainGameMode (Game|GetGameMode)))
                (Default|UpdateHealth (Variables|/Game/GameSettings/MainGameMode.MainGameMode_C|GetHeadsUpDisplay _asmain_game_mode))))))))))

(fn ConstructionScript)