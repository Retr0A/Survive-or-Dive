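; Shooter is a trap-like actor that fires when the player character crosses its line of sight.
; Each Tick it sphere-traces forward from its Scene component on the Camera channel and calls ShootArrrow if the hit actor is the player.
; ShootArrrow spawns an actor at the Scene transform with a shooting sound, throttled by a DoOnce that resets after a short delay.
; A looping timer for periodic firing is left unconnected.
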(event Custom|ShootArrrow
  (Utilities|FlowControl|DoOnce false :!label _label
    (:Completed
      (Game|SpawnActorfromClass "/Game/Blueprints/Arrow.Arrow_C" (Transformation|GetWorldTransform (Variables|Default|GetScene)) "Undefined" 0 0)
      (Audio|PlaySoundatLocation "/Game/Sounds/Shooting.Shooting" (Transformation|GetActorLocation) "0, 0, 0" 1.0 1.0 0.0 0 0 0)
      (Utilities|FlowControl|Delay 2.0)
      (goto _label Reset))))

(event EventBeginPlay)

(event Collision|EventActorBeginOverlap
  (params (OtherActor :type Actor%20Object%20Reference)))

(event EventTick
  (params (DeltaSeconds :type Float%20%28single-precision%29))
  (bind _scene (Variables|Default|GetScene))
  (bind _returnvalue (Transformation|GetWorldLocation _scene))
  (bind _outhit (Collision|SphereTraceByChannel _returnvalue (+ _returnvalue (* (Math|Vector|GetForwardVector (Transformation|GetWorldRotation _scene)) 3000)) 1e+01 "TraceTypeQuery2" false 0 "None"))
  (if (== (.HitActor (Collision|BreakHitResult _outhit)) (Game|GetPlayerCharacter 0))
    (CallFunction|ShootArrrow)))

(fn ConstructionScript)