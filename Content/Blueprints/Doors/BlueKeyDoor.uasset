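; Door actor that the player opens by spending one blue key.
; A trigger overlap enables input while the door is closed and shows either an interact prompt or a key-required message through the game mode's HUD; leaving disables input.
; Interacting decrements the key count, refreshes the HUD, attaches a spawned key mesh to the keyhole and plays a sound.
; A timeline then moves the door along Z and marks it open on finish.
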(event OnComponentBeginOverlap(Trigger)
  (params (OverlappedComponent :type Primitive%20Component%20Object%20Reference) (OtherActor :type Actor%20Object%20Reference) (OtherComp :type Primitive%20Component%20Object%20Reference) (OtherBodyIndex :type Integer) (bFromSweep :type Boolean) (SweepResult :type Hit%20Result%20Structure%20%28by%20ref%29))
  (bind _returnvalue (Game|GetPlayerController 0))
  (if (== OtherActor (Game|GetPlayerCharacter 0))
    (if (not (Variables|Default|GetIsOpen))
      (bind _asplayer_character (Utilities|Casting|CastToPlayerCharacter (Game|GetPlayerCharacter 0)))
      (if (> (Variables|/Game/Characters/PlayerCharacter.PlayerCharacter_C|GetNumberOfBlueKeys _asplayer_character) 0)
        (Input|EnableInput _returnvalue)
        (bind _asmain_game_mode (Utilities|Casting|CastToMainGameMode (Game|GetGameMode)))
        (Variables|/Game/UI/HeadsUpDisplay.HeadsUpDisplay_C|SetMessage (Variables|/Game/GameSettings/MainGameMode.MainGameMode_C|GetHeadsUpDisplay _asmain_game_mode) "Press [E] to open the door.")
        (Default|UpdateMessage (Variables|/Game/GameSettings/MainGameMode.MainGameMode_C|GetHeadsUpDisplay _asmain_game_mode))
        (else
          (Input|EnableInput _returnvalue)
          (bind _asmain_game_mode_2 (Utilities|Casting|CastToMainGameMode (Game|GetGameMode)))
          (Variables|/Game/UI/HeadsUpDisplay.HeadsUpDisplay_C|SetMessage (Variables|/Game/GameSettings/MainGameMode.MainGameMode_C|GetHeadsUpDisplay _asmain_game_mode_2) "You need a blue key to open the door.")
          (Default|UpdateMessage (Variables|/Game/GameSettings/MainGameMode.MainGameMode_C|GetHeadsUpDisplay _asmain_game_mode_2)))))))

(event OnComponentEndOverlap(Trigger)
  (params (OverlappedComponent :type Primitive%20Component%20Object%20Reference) (OtherActor :type Actor%20Object%20Reference) (OtherComp :type Primitive%20Component%20Object%20Reference) (OtherBodyIndex :type Integer))
  (if (== OtherActor (Game|GetPlayerCharacter 0))
    (Input|DisableInput (Game|GetPlayerController 0))
    (bind _asmain_game_mode (Utilities|Casting|CastToMainGameMode (Game|GetGameMode)))
    (Variables|/Game/UI/HeadsUpDisplay.HeadsUpDisplay_C|SetMessage (Variables|/Game/GameSettings/MainGameMode.MainGameMode_C|GetHeadsUpDisplay _asmain_game_mode) "")
    (Default|UpdateMessage (Variables|/Game/GameSettings/MainGameMode.MainGameMode_C|GetHeadsUpDisplay _asmain_game_mode))))

(event EventBeginPlay)

(event Collision|EventActorBeginOverlap
  (params (OtherActor :type Actor%20Object%20Reference)))

(event EventTick
  (params (DeltaSeconds :type Float%20%28single-precision%29)))

(event Input|ActionEvents|InputActionInteract
  (params (Key :type Key%20Structure :default "None"))
  (:Pressed
    (bind _asplayer_character (Utilities|Casting|CastToPlayerCharacter (Game|GetPlayerCharacter 0)))
    (if (> (Variables|/Game/Characters/PlayerCharacter.PlayerCharacter_C|GetNumberOfBlueKeys _asplayer_character) 0)
      (Math|Integer|DecrementInt (Variables|/Game/Characters/PlayerCharacter.PlayerCharacter_C|GetNumberOfBlueKeys _asplayer_character)
        (:%20%20
          (bind _asmain_game_mode (Utilities|Casting|CastToMainGameMode (Game|GetGameMode)))
          (Default|UpdateKeys (Variables|/Game/GameSettings/MainGameMode.MainGameMode_C|GetHeadsUpDisplay _asmain_game_mode))
          (bind _returnvalue (AddComponent|AddStaticMeshComponent false))
          (bind _output_get (Variables|Default|SetKeyMesh _returnvalue))
          (Transformation|AttachComponentToComponent _output_get (Variables|Default|GetKeyhole) "None" "KeepRelative" "KeepRelative" "KeepRelative" true)
          (Audio|PlaySoundatLocation "/Game/Sounds/DoorOpening.DoorOpening" (Transformation|GetActorLocation) "0, 0, 0" 1.0 1.0 0.0 0 0 0)
          (bind _doorposition (Timeline|Anim Play)
            (:Update
              (Transformation|SetRelativeLocation (Variables|Default|GetMesh) (Math|Vector|MakeVector 0.0 0.0 _doorposition) false false))
            (:Finished
              (Variables|Default|SetIsOpen true)
              (bind _asmain_game_mode_2 (Utilities|Casting|CastToMainGameMode (Game|GetGameMode)))
              (Variables|/Game/UI/HeadsUpDisplay.HeadsUpDisplay_C|SetMessage (Variables|/Game/GameSettings/MainGameMode.MainGameMode_C|GetHeadsUpDisplay _asmain_game_mode_2) "")
              (Default|UpdateMessage (Variables|/Game/GameSettings/MainGameMode.MainGameMode_C|GetHeadsUpDisplay _asmain_game_mode_2)))))))))

(fn ConstructionScript)