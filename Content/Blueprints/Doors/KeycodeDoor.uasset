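; Keycode-locked door that prompts the player inside its trigger to interact, then slides open vertically when a valid code has been entered.
; Trigger overlaps toggle input and the HUD message.
; Interact passes the door's code to the HUD keypad, shows it, and checks validity in that same press without waiting for entry.
; On success, a timeline moves the mesh with sound; leftover gold-key logic is disconnected.
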(event OnComponentBeginOverlap(Trigger)
  (params (OverlappedComponent :type Primitive%20Component%20Object%20Reference) (OtherActor :type Actor%20Object%20Reference) (OtherComp :type Primitive%20Component%20Object%20Reference) (OtherBodyIndex :type Integer) (bFromSweep :type Boolean) (SweepResult :type Hit%20Result%20Structure%20%28by%20ref%29))
  (if (== OtherActor (Game|GetPlayerCharacter 0))
    (if (not (Variables|Default|GetIsOpen))
      (bind _asplayer_character (Utilities|Casting|CastToPlayerCharacter (Game|GetPlayerCharacter 0)))
      (Input|EnableInput (Game|GetPlayerController 0))
      (bind _asmain_game_mode (Utilities|Casting|CastToMainGameMode (Game|GetGameMode)))
      (Variables|/Game/UI/HeadsUpDisplay.HeadsUpDisplay_C|SetMessage (Variables|/Game/GameSettings/MainGameMode.MainGameMode_C|GetHeadsUpDisplay _asmain_game_mode) "Press [E] to enter the key.")
      (Default|UpdateMessage (Variables|/Game/GameSettings/MainGameMode.MainGameMode_C|GetHeadsUpDisplay _asmain_game_mode)))))

(event OnComponentEndOverlap(Trigger)
  (params (OverlappedComponent :type Primitive%20Component%20Object%20Reference) (OtherActor :type Actor%20Object%20Reference) (OtherComp :type Primitive%20Component%20Object%20Reference) (OtherBodyIndex :type Integer))
  (if (== OtherActor (Game|GetPlayerCharacter 0))
    (Input|DisableInput (Game|GetPlayerController 0))
    (bind _asmain_game_mode (Utilities|Casting|CastToMainGameMode (Game|GetGameMode)))
    (Variables|/Game/UI/HeadsUpDisplay.HeadsUpDisplay_C|SetMessage (Variables|/Game/GameSettings/MainGameMode.MainGameMode_C|GetHeadsUpDisplay _asmain_game_mode) "")
    (Default|UpdateMessage (Variables|/Game/GameSettings/MainGameMode.MainGameMode_C|GetHeadsUpDisplay _asmain_game_mode))))

(event EventBeginPlay)

(event Collision|EventActorBeginOverlap
  (params (OtherActor :type Actor%20Object%20Reference)))

(event EventTick
  (params (DeltaSeconds :type Float%20%28single-precision%29)))

(event Input|ActionEvents|InputActionInteract
  (params (Key :type Key%20Structure :default "None"))
  (bind _returnvalue (Game|GetGameMode))
  (bind _returnvalue_2 (Game|GetPlayerController 0))
  (bind _asmain_game_mode (Utilities|Casting|CastToMainGameMode _returnvalue))
  (bind _headsupdisplay (Variables|/Game/GameSettings/MainGameMode.MainGameMode_C|GetHeadsUpDisplay _asmain_game_mode))
  (:Pressed
    (Variables|Default|SetKeycodeUI (Variables|/Game/UI/HeadsUpDisplay.HeadsUpDisplay_C|GetKeycodeUI _headsupdisplay))
    (Variables|/Game/UI/KeycodeUI.KeycodeUI_C|SetKeycode (Variables|/Game/UI/HeadsUpDisplay.HeadsUpDisplay_C|GetKeycodeUI _headsupdisplay) (Variables|Default|GetKeyCode))
    (Widget|SetVisibility (Variables|/Game/UI/HeadsUpDisplay.HeadsUpDisplay_C|GetKeycodeUI _headsupdisplay) "Visible")
    (Input|SetInputModeUIOnly _returnvalue_2 _headsupdisplay "DoNotLock")
    (Variables|/Script/Engine.PlayerController|SetbShowMouseCursor _returnvalue_2 true)
    (if (and (== (Variables|/Game/UI/KeycodeUI.KeycodeUI_C|GetKeycode (Variables|Default|GetKeycodeUI)) (Variables|Default|GetKeyCode)) (Variables|/Game/UI/KeycodeUI.KeycodeUI_C|GetIsValidKeycode (Variables|Default|GetKeycodeUI)))
      (Audio|PlaySoundatLocation "/Game/Sounds/DoorOpening.DoorOpening" (Transformation|GetActorLocation) "0, 0, 0" 1.0 1.0 0.0 0 0 0)
      (bind _doorposition (Timeline|Anim PlayFromStart)
        (:Update
          (Transformation|SetRelativeLocation (Variables|Default|GetMesh) (Math|Vector|MakeVector 0.0 0.0 _doorposition) false true))
        (:Finished
          (Variables|Default|SetIsOpen true)
          (bind _asmain_game_mode_2 (Utilities|Casting|CastToMainGameMode (Game|GetGameMode)))
          (Variables|/Game/UI/HeadsUpDisplay.HeadsUpDisplay_C|SetMessage (Variables|/Game/GameSettings/MainGameMode.MainGameMode_C|GetHeadsUpDisplay _asmain_game_mode_2) "")
          (Default|UpdateMessage (Variables|/Game/GameSettings/MainGameMode.MainGameMode_C|GetHeadsUpDisplay _asmain_game_mode_2)))))))

(fn ConstructionScript)