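; Blue key pickup actor that the player collects by pressing Interact while inside its Box trigger.
; Box overlap enables or disables the actor's input and sets or clears the HUD prompt through MainGameMode.
; Interact increments the player's blue key count, refreshes the HUD key display and plays a pickup sound.
; Only the static mesh is destroyed; its validity gates the prompt and prevents repeat pickups.
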(event OnComponentBeginOverlap(Box)
  (params (OverlappedComponent :type Primitive%20Component%20Object%20Reference) (OtherActor :type Actor%20Object%20Reference) (OtherComp :type Primitive%20Component%20Object%20Reference) (OtherBodyIndex :type Integer) (bFromSweep :type Boolean) (SweepResult :type Hit%20Result%20Structure%20%28by%20ref%29))
  (if (== OtherActor (Game|GetPlayerCharacter 0))
    (Input|EnableInput (Game|GetPlayerController 0))
    (Utilities|IsValid (Variables|Default|GetStaticMesh)
      (:Is%20Valid
        (bind _asmain_game_mode (Utilities|Casting|CastToMainGameMode (Game|GetGameMode)))
        (Variables|/Game/UI/HeadsUpDisplay.HeadsUpDisplay_C|SetMessage (Variables|/Game/GameSettings/MainGameMode.MainGameMode_C|GetHeadsUpDisplay _asmain_game_mode) "Press [E] to pick up the key.")
        (Default|UpdateMessage (Variables|/Game/GameSettings/MainGameMode.MainGameMode_C|GetHeadsUpDisplay _asmain_game_mode))))))

(event OnComponentEndOverlap(Box)
  (params (OverlappedComponent :type Primitive%20Component%20Object%20Reference) (OtherActor :type Actor%20Object%20Reference) (OtherComp :type Primitive%20Component%20Object%20Reference) (OtherBodyIndex :type Integer))
  (if (== OtherActor (Game|GetPlayerCharacter 0))
    (Input|DisableInput (Game|GetPlayerController 0))
    (bind _asmain_game_mode (Utilities|Casting|CastToMainGameMode (Game|GetGameMode)))
    (Variables|/Game/UI/HeadsUpDisplay.HeadsUpDisplay_C|SetMessage (Variables|/Game/GameSettings/MainGameMode.MainGameMode_C|GetHeadsUpDisplay _asmain_game_mode) "")
    (Default|UpdateMessage (Variables|/Game/GameSettings/MainGameMode.MainGameMode_C|GetHeadsUpDisplay _asmain_game_mode))))

(event EventBeginPlay)

(event Collision|EventActorBeginOverlap
  (params (OtherActor :type Actor%20Object%20Reference)))

(event EventTick
  (params (DeltaSeconds :type Float%20%28single-precision%29)))

(event Input|ActionEvents|InputActionInteract
  (params (Key :type Key%20Structure :default "None"))
  (bind _staticmesh (Variables|Default|GetStaticMesh))
  (:Pressed
    (Utilities|IsValid _staticmesh
      (:Is%20Valid
        (bind _asplayer_character (Utilities|Casting|CastToPlayerCharacter (Game|GetPlayerCharacter 0)))
        (Math|Integer|IncrementInt (Variables|/Game/Characters/PlayerCharacter.PlayerCharacter_C|GetNumberOfBlueKeys _asplayer_character)
          (:%20%20
            (Components|DestroyComponent _staticmesh)
            (bind _asmain_game_mode (Utilities|Casting|CastToMainGameMode (Game|GetGameMode)))
            (Default|UpdateKeys (Variables|/Game/GameSettings/MainGameMode.MainGameMode_C|GetHeadsUpDisplay _asmain_game_mode))
            (Audio|PlaySoundatLocation "/Game/Sounds/Pickup.Pickup" (Transformation|GetActorLocation (Game|GetPlayerCharacter 0)) "0, 0, 0" 1.0 1.0 0.0 0 0 0)))))))

(fn ConstructionScript)